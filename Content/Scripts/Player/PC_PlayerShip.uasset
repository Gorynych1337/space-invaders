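; Player-controlled ship for a flipbook-sprite shooter, handling side movement, automatic fire, damage and pausing.
; Enhanced Input drives lateral movement, with left, right or forward flipbooks chosen from X velocity.
; A Delay on Tick paces continuous twin projectile spawns from two arrow components.
; Hits go through ACPlayerStats to trigger death and open the Space level, while pause toggles the HUD widget and cursor.
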(event `self.ReceiveBeginPlay`
  (bind _returnvalue (pcsubsystem `EnhancedInputLocalPlayerSubsystem` (`GameplayStatics.GetPlayerController` 0)))
  ;[1 1 1] Add Input System
  (`/Engine/EditorBlueprintResources/StandardMacros.IsValid` _returnvalue
    (:`Is Valid`
      (`EnhancedInputSubsystemInterface.AddMappingContext` _returnvalue "/Game/Scripts/Inputs/IMC_Inputs.IMC_Inputs" 0 (struct)))))

(event `EnhancedInput|/Game/Scripts/Inputs/IA_SideMove`
  (params (ActionValue :type "Float (double-precision)") (ElapsedSeconds :type "Float (double-precision)") (TriggeredSeconds :type "Float (double-precision)") (InputAction :type "InputAction Object Reference" :default "/Game/Scripts/Inputs/IA_SideMove.IA_SideMove"))
  (bind _sprite (`self.Sprite`))
  (bind _isdead (`self.IsDead`))
  ;[1 1 1] Movement
  (:`Triggered`
    (if (not _isdead)
      (`self.AddMovementInput` (1.0 0.0 0.0) ActionValue)
      (`/Engine/EditorBlueprintResources/StandardMacros.CompareFloat` (.x (`self.GetVelocity`))
        (:`>`
          (`PaperFlipbookComponent.SetFlipbook` _sprite "/Game/Assets/Ship/ShipRight.ShipRight"))
        (:`==`
          (`PaperFlipbookComponent.SetFlipbook` _sprite "/Game/Assets/Ship/ShipForward.ShipForward" :!label _label))
        (:`<`
          (`PaperFlipbookComponent.SetFlipbook` _sprite "/Game/Assets/Ship/ShipLeft.ShipLeft")))))
  (:`Completed`
    (if (not _isdead)
      (goto _label))))

(event `self.ReceiveTick`
  (params (DeltaSeconds :type "Float (single-precision)"))
  ;[1 1 1] Shoot
  (`KismetSystemLibrary.Delay` (`self.ShotDelay`))
  (`self.SpawnProjectile` "/Game/Scripts/BC_Shot.BC_Shot_C" (`self.LeftShotArrow`))
  (`self.SpawnProjectile` "/Game/Scripts/BC_Shot.BC_Shot_C" (`self.RightShotArrow`)))

(event `/Game/Scripts/IHittable.On Hit`
  ;[1 1 1] OnHit
  (bind _isdead (`/Game/Scripts/Player/AC_PlayerStats.DegreesHP` (`self.AC_PlayerStats`)))
  (if _isdead
    (set `self.IsDead` true)
    (`parent.On Hit`)
    (`GameplayStatics.OpenLevelBySoftObjectPtr` "/Game/Levels/Space.Space")))

(event `EnhancedInput|/Game/Scripts/Inputs/IA_Pause`
  (params (ActionValue :type Boolean) (ElapsedSeconds :type "Float (double-precision)") (TriggeredSeconds :type "Float (double-precision)") (InputAction :type "InputAction Object Reference" :default "/Game/Scripts/Inputs/IA_Pause.IA_Pause"))
  (bind _returnvalue (`GameplayStatics.IsGamePaused`))
  ;[1 1 1] Pause
  (:`Triggered`
    (bind _asbc_hud (cast `/Game/Scripts/Player/BC_HUD` (`PlayerController.GetHUD` (`GameplayStatics.GetPlayerController` 0))))
    (`/Game/Scripts/Player/BC_HUD.SetWidget` _asbc_hud (select `bool` _returnvalue :`false` "NewEnumerator1" :`true` "NewEnumerator0" :!type "/Game/Scripts/Player/EHUDs Enum"))
    (`GameplayStatics.SetGamePaused` (not _returnvalue))
    (set `PlayerController.bShowMouseCursor` _returnvalue (`GameplayStatics.GetPlayerController` 0))))

(fn `UserConstructionScript`)