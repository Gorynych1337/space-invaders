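; AC_PlayerStats is a player stats component that tracks HP and score.
; On BeginPlay it caches the first player controller's HUD as BC_HUD.
; DegreesHP lowers HP by one, tells the HUD to remove that HP and returns whether HP has reached zero.
; AddScore adds the given points to Score without updating the HUD.
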(event `self.ReceiveBeginPlay`
  (bind _asbc_hud (cast `/Game/Scripts/Player/BC_HUD` (`PlayerController.GetHUD` (`GameplayStatics.GetPlayerController` 0))))
  (set `self.HUD` _asbc_hud))

(fn `AddScore`
  (params (Points :type Integer))
  (set `self.Score` (+ Points (`self.Score`))))

(fn `DegreesHP`
  (returns (IsDead :type Boolean))
  (bind _output_get (set `self.HP` (- (`self.HP`) 1)))
  (`/Game/Scripts/Player/BC_HUD.RemoveHP` (`self.HUD`) _output_get)
  (return (== _output_get 0)))