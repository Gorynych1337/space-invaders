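; UFO enemy that shoots projectiles and awards points to the player when hit.
; Its OnHit override uses a one-time flag, adds its point value through the player ship's stats component, runs the parent hit logic, then fires the UfoDestroyed dispatcher with itself.
; Shoot spawns a UFO shot at the arrow component's location.
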(event `/Game/Scripts/IHittable.On Hit`
  ;[1 1 1] OnHit overwritting
  (if (not (`self.IsHitted`))
    (set `self.IsHitted` true)
    (bind _aspc_player_ship (cast `/Game/Scripts/Player/PC_PlayerShip` (`GameplayStatics.GetPlayerCharacter` 0)))
    (`/Game/Scripts/Player/AC_PlayerStats.AddScore` (`/Game/Scripts/Player/PC_PlayerShip.AC_PlayerStats` _aspc_player_ship) (`self.PointValue`))
    (`parent.On Hit`)
    (`self.UfoDestroyed` self)))

(fn `Shoot`
  (`self.SpawnProjectile` "/Game/Scripts/BC_UfoShot.BC_UfoShot_C" (`self.ShotArrow`)))

(fn `UserConstructionScript`)